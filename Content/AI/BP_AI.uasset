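; AI-controlled pawn Blueprint that spots the player and performs a melee shove attack.
; PawnSensing sets the seeingPlayer Blackboard key when it sees a Player-tagged pawn, and nothing here clears it.
; AttackPlayer plays a montage, immediately sphere-traces forward from AttackTracePoint for pawns, and damages any hit.
; An Attacking flag gates the attack and clears on montage completion, but is never set true here.
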(event OnSeePawn(PawnSensing)
  (params (Pawn :type Pawn%20Object%20Reference))
  (if (Actor|ActorHasTag Pawn "Player")
    (AI|Components|Blackboard|SetValueasBool (AI|GetBlackboard (AI|GetAIController self)) (Utilities|Name|MakeLiteralName "seeingPlayer") true)))

(event Custom|Attack%20Player
  (bind _attack_trace_point (Variables|Default|GetAttack%20Trace%20Point))
  (bind _returnvalue (Transformation|GetWorldLocation _attack_trace_point))
  (if (not (Variables|Default|GetAttacking?))
    (Animation|Montage|PlayMontage (Variables|Character|GetMesh) "/Game/AI/Paired_PushShove_Att_Montage.Paired_PushShove_Att_Montage"
      (:then
        (bind (_outhit _returnvalue_2) (Collision|SphereTraceForObjects _returnvalue (+ (* (Math|Vector|GetForwardVector (Transformation|GetWorldRotation _attack_trace_point)) 7e+01) _returnvalue) 25.0 (Utilities|Array|MakeArray "ObjectTypeQuery3") false 0 "ForDuration"))
        (if _returnvalue_2
          (Game|Damage|ApplyDamage (.HitActor (Collision|BreakHitResult _outhit)) 1e+01 0 0)))
      (:OnCompleted
        (Variables|Default|SetAttacking? false)))))

(event EventBeginPlay)

(event Collision|EventActorBeginOverlap
  (params (OtherActor :type Actor%20Object%20Reference)))

(event EventTick
  (params (DeltaSeconds :type Float%20%28single-precision%29)))

(fn ConstructionScript)