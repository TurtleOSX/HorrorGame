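; BP_Drawer is an enterable drawer that moves the player in and out when interacted with.
; Interact toggles an Inside flag, snapping player character 0 to the ReferenceInside or ReferenceOutside transform's location and rotation.
; The Door rotates shut on entry and swings open on exit, both instantly without animation.
; Overlap by BP_ThirdPersonCharacter only prints a debug "Hello".
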(event EventBeginPlay)

(event Collision|EventActorBeginOverlap
  (params (OtherActor :type Actor%20Object%20Reference))
  (Utilities|Casting|CastToBP_ThirdPersonCharacter OtherActor)
  (Development|PrintString "Hello"))

(event EventTick
  (params (DeltaSeconds :type Float%20%28single-precision%29)))

(event EventInteract
  (bind _referenceinside (Variables|Default|GetReferenceInside))
  (bind _referenceoutside (Variables|Default|GetReferenceOutside))
  (bind _returnvalue (Transformation|GetWorldTransform _referenceinside))
  (bind _returnvalue_2 (Transformation|GetWorldTransform _referenceoutside))
  (if (not (Variables|Default|GetInside))
    (Variables|Default|SetInside true)
    (Transformation|SetActorTransform (Game|GetPlayerCharacter 0) (Math|Transform|MakeTransform (.location _returnvalue) (.rotation _returnvalue) "1.000000,1.000000,1.000000"))
    (Transformation|SetRelativeRotation (Variables|Default|GetDoor) "0, 0, 0" false false)
    (else
      (Variables|Default|SetInside false)
      (Transformation|SetActorTransform (Game|GetPlayerCharacter 0) (Math|Transform|MakeTransform (.location _returnvalue_2) (.rotation _returnvalue_2) "1.000000,1.000000,1.000000"))
      (Transformation|SetRelativeRotation (Variables|Default|GetDoor) "0.000000,109.999999,0.000000" false false))))

(fn ConstructionScript)