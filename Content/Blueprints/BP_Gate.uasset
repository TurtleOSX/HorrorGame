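; Double gate actor that stays shut until all collectables are gathered, then serves as the level's win exit.
; A Box trigger enables the gate's input for BP_FirstPerson, so Interact checks CollectablesLeft on BP_ThirdPersonGameMode and plays a timeline swinging both leaves open.
; Overlapping the WinCheck trigger disables player input, shows the win widget and loads the main menu after a short delay.
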(event OnComponentBeginOverlap(Box)
  (params (OverlappedComponent :type Primitive%20Component%20Object%20Reference) (OtherActor :type Actor%20Object%20Reference) (OtherComp :type Primitive%20Component%20Object%20Reference) (OtherBodyIndex :type Integer) (bFromSweep :type Boolean) (SweepResult :type Hit%20Result%20Structure%20%28by%20ref%29))
  (Utilities|Casting|CastToBP_FirstPerson OtherActor)
  (Input|EnableInput (Game|GetPlayerController 0)))

(event OnComponentEndOverlap(Box)
  (params (OverlappedComponent :type Primitive%20Component%20Object%20Reference) (OtherActor :type Actor%20Object%20Reference) (OtherComp :type Primitive%20Component%20Object%20Reference) (OtherBodyIndex :type Integer))
  (Utilities|Casting|CastToBP_FirstPerson OtherActor)
  (Input|DisableInput (Game|GetPlayerController 0)))

(event OnComponentBeginOverlap(WinCheck)
  (params (OverlappedComponent :type Primitive%20Component%20Object%20Reference) (OtherActor :type Actor%20Object%20Reference) (OtherComp :type Primitive%20Component%20Object%20Reference) (OtherBodyIndex :type Integer) (bFromSweep :type Boolean) (SweepResult :type Hit%20Result%20Structure%20%28by%20ref%29))
  (bind _asbp_first_person (Utilities|Casting|CastToBP_FirstPerson OtherActor))
  (Input|DisableInput _asbp_first_person (Game|GetPlayerController 0))
  (Utilities|Casting|CastToBP_ThirdPersonGameMode (Game|GetGameMode))
  (bind _returnvalue (UserInterface|CreateWidget "/Game/UI/WB_Win.WB_Win_C"))
  (UserInterface|Viewport|AddtoViewport _returnvalue 0)
  (Utilities|FlowControl|Delay 2.0)
  (Game|OpenLevel(byObjectReference) "/Game/MainMenu/MainMenuLevel.MainMenuLevel"))

(event Input|EnhancedActionEvents|EnhancedInputActionIA_Interact
  (params (ActionValue :type Boolean) (ElapsedSeconds :type Float%20%28double-precision%29) (TriggeredSeconds :type Float%20%28double-precision%29) (InputAction :type Input%20Action%20Object%20Reference :default "/Game/ThirdPerson/Input/Actions/IA_Interact.IA_Interact"))
  (:Started
    (bind _asbp_third_person_game_mode (Utilities|Casting|CastToBP_ThirdPersonGameMode (Game|GetGameMode)))
    (if (== (Variables|/Game/ThirdPerson/Blueprints/BP_ThirdPersonGameMode.BP_ThirdPersonGameMode_C|GetCollectables%20Left _asbp_third_person_game_mode) 0)
      (bind _open_close (Timeline|Open%20Gate Play)
        (:Update
          (Transformation|SetRelativeRotation (Variables|Default|GetLeftGate) (Math|Rotator|MakeRotator 0.0 0.0 (Math|Float|Lerp 0.0 -9e+01 _open_close)) false false)
          (Transformation|SetRelativeRotation (Variables|Default|GetRightGate) (Math|Rotator|MakeRotator 0.0 0.0 (Math|Float|Lerp 1.8e+02 2.7e+02 _open_close)) false false))))))

(fn ConstructionScript)