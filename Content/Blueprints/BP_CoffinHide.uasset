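; BP_CoffinHide is a coffin hiding spot that the player can enter and leave through an Interact event.
; Each interaction toggles Inside, teleporting the player to the InnerRef or OuterRef transform and snapping the Door between two hardcoded relative transforms without animation.
; It also sets IsHiding on BP_FirstPerson to match.
; The overlap event only casts to BP_FirstPerson and has no further effect.
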(event Collision|EventActorBeginOverlap
  (params (OtherActor :type Actor%20Object%20Reference))
  ;[0.1979 0.1979 0.1979] Begin Actor Overlap
  (Utilities|Casting|CastToBP_FirstPerson OtherActor))

(event EventInteract
  (bind _returnvalue (Game|GetPlayerCharacter 0))
  (bind _innerref (Variables|Default|GetInnerRef))
  (bind _outerref (Variables|Default|GetOuterRef))
  (bind _returnvalue_2 (Transformation|GetWorldTransform _innerref))
  (bind _returnvalue_3 (Transformation|GetWorldTransform _outerref))
  ;[0.1615 0.1615 0.1615] Interact
  (if (not (Variables|Default|GetInside))
    (Variables|Default|SetInside true)
    (Transformation|SetActorTransform (Game|GetPlayerCharacter 0) (Math|Transform|MakeTransform (.location _returnvalue_2) (.rotation _returnvalue_2) "1.000000,1.000000,1.000000"))
    (Transformation|SetRelativeTransform (Variables|Default|GetDoor) (Math|Transform|MakeTransform "0.000000,40.000000,110.000000" "0.000000,0.000000,90.000000" "1.000000,1.000000,1.000000") false false)
    (bind _asbp_first_person (Utilities|Casting|CastToBP_FirstPerson _returnvalue))
    (Variables|/Game/Blueprints/BP_FirstPerson.BP_FirstPerson_C|SetisHiding _asbp_first_person true)
    (else
      (Variables|Default|SetInside false)
      (Transformation|SetActorTransform (Game|GetPlayerCharacter 0) (Math|Transform|MakeTransform (.location _returnvalue_3) (.rotation _returnvalue_3) "1.000000,1.000000,1.000000"))
      (Transformation|SetRelativeTransform (Variables|Default|GetDoor) (Math|Transform|MakeTransform "-45.000000,40.000000,110.000000" "0.000000,40.000000,90.000000" "1.000000,1.000000,1.000000") false false)
      (bind _asbp_first_person_2 (Utilities|Casting|CastToBP_FirstPerson _returnvalue))
      (Variables|/Game/Blueprints/BP_FirstPerson.BP_FirstPerson_C|SetisHiding _asbp_first_person_2 false))))

(fn ConstructionScript)